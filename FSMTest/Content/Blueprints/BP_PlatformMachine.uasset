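; Demo actor that cycles a FiniteStateMachine component through sleeping, eating, MyStateObject and slicing states, starting asleep on BeginPlay.
; Tick compares the current state's class behind a short Delay, then further Delays time most transitions.
; The sleeping, eating and slicing branches each move the Cube to a different relative location.
; The MyStateObject and slicing branches print the machine's message, and MyStateObject switches to slicing without an extra wait.
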(event EventBeginPlay
  (Class|FiniteStateMachine|ChangeState (Variables|Default|GetFiniteStateMachine) "/Script/FSMTest.SleepingState"))

(event Collision|EventActorBeginOverlap
  (params (OtherActor :type Actor%20Object%20Reference)))

(event EventTick
  (params (DeltaSeconds :type Float%20%28single-precision%29))
  (Utilities|FlowControl|Delay 0.2)
  (bind _returnvalue (Class|FiniteStateMachine|GetState (Variables|Default|GetFiniteStateMachine)))
  (if (== (Variables|Default|GetsleepingState) (Utilities|GetClass _returnvalue))
    (Transformation|SetRelativeLocation (Variables|Default|GetCube) "0,20.000000, 0" false false)
    (Utilities|FlowControl|Delay 4.0)
    (Class|FiniteStateMachine|ChangeState (Variables|Default|GetFiniteStateMachine) "/Script/FSMTest.EatingState")
    (elif (== (Utilities|GetClass _returnvalue) (Variables|Default|GetMyStateObject))
      (bind _returnvalue_2 (Class|FiniteStateMachine|GetMessage (Variables|Default|GetFiniteStateMachine)))
      (Development|PrintString (Utilities|String|ToString(Text) _returnvalue_2) true true "(R=0.000000,G=0.660000,B=1.000000,A=1.000000)" 5.0)
      (Class|FiniteStateMachine|ChangeState (Variables|Default|GetFiniteStateMachine) "/Game/Blueprints/SlicingState.SlicingState_C")
      (elif (== (Variables|Default|GetslicingState) (Utilities|GetClass _returnvalue))
        (Transformation|SetRelativeLocation (Variables|Default|GetCube) "0, 0,10.000000" false false)
        (bind _returnvalue_3 (Class|FiniteStateMachine|GetMessage (Variables|Default|GetFiniteStateMachine)))
        (Development|PrintString (Utilities|String|ToString(Text) _returnvalue_3))
        (Utilities|FlowControl|Delay 2.0)
        (Class|FiniteStateMachine|ChangeState (Variables|Default|GetFiniteStateMachine) "/Script/FSMTest.SleepingState")
        (else
          (Transformation|SetRelativeLocation (Variables|Default|GetCube) "0,-20.000000, 0" false false)
          (Utilities|FlowControl|Delay 4.0)
          (Class|FiniteStateMachine|ChangeState (Variables|Default|GetFiniteStateMachine) "/Game/Blueprints/MyStateObject.MyStateObject_C"))))))

(fn ConstructionScript)